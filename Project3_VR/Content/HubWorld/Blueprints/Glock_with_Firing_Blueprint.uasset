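; VR Glock pistol that is picked up by a motion controller and fires hitscan shots.
; Pickup disables physics and snaps the gun to the controller with an offset; Drop detaches it and restores physics.
; The holding hand's trigger runs a debug-drawn line trace from an Arrow, dealing point damage, playing a shot sound at impact and pushing physics objects.
; Firing never checks PickedUp, and the impulse vector reuses the impact position.
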(event Collision|EventActorBeginOverlap
  (params (OtherActor :type Actor%20Object%20Reference)))

(event EventTick
  (params (DeltaSeconds :type Float%20%28single-precision%29)))

(event EventPickup
  (params (AttachTo :type Scene%20Component%20Object%20Reference))
  (if (Utilities|IsValid AttachTo)
    (bind _asmotion_controller_component (Utilities|Casting|CastToMotionControllerComponent AttachTo))
    (Variables|Default|Setpicked_up true)
    (Physics|SetSimulatePhysics (Variables|SkeletalMeshActor|GetSkeletalMeshComponent) false)
    (Transformation|AttachComponentToComponent (VehicleSound|GetRootComponent) AttachTo "None" "SnapToTarget" "SnapToTarget" "KeepWorld" false)
    (Transformation|SetRelativeLocationAndRotation (Variables|SkeletalMeshActor|GetSkeletalMeshComponent) "3.000000,0.000000,-2.000000" "-20.000000,0.000000,90.000000" false false)))

(event EventDrop
  (Variables|Default|Setpicked_up false)
  (Physics|SetSimulatePhysics (Variables|SkeletalMeshActor|GetSkeletalMeshComponent) true)
  (Transformation|DetachFromActor "KeepWorld" "KeepWorld" "KeepWorld"))

(event Input|KeyboardEvents|MotionControllerRightTrigger
  (params (Key :type Key%20Structure))
  (bind _arrow (Variables|Default|GetArrow))
  (bind _returnvalue (Transformation|GetWorldLocation _arrow))
  (:Pressed
    (if (Utilities|IsValid (stale EventPickup AttachTo))
      (if (Utilities|Name|Equal(Name) (Variables|/Script/HeadMountedDisplay.MotionControllerComponent|GetMotionSource (stale EventPickup _asmotion_controller_component)) "EControllerHand::Right")
        (if true
          (bind (_outhit _returnvalue_2) (Collision|LineTraceByChannel _returnvalue (+ _returnvalue (* (Math|Vector|GetForwardVector _arrow) 3e+03)) "TraceTypeQuery1" false 0 "ForDuration"))
          (if _returnvalue_2
            (Game|Damage|ApplyPointDamage (.HitActor (Collision|BreakHitResult _outhit)) 1.0 (.ImpactPoint (Collision|BreakHitResult _outhit)) _outhit)
            (Audio|PlaySoundatLocation "/Game/MiniGame1/Audio/Sound_Effects/Beretta_M9.Beretta_M9" (.ImpactPoint (Collision|BreakHitResult _outhit)) "0, 0, 0" 0.2 1.0 0.0 0 0 0)
            (if (Physics|IsSimulatingPhysics (.HitComponent (Collision|BreakHitResult _outhit)) "None")
              (Physics|AddImpulseatLocation (.HitComponent (Collision|BreakHitResult _outhit)) (.ImpactPoint (Collision|BreakHitResult _outhit)) (.ImpactPoint (Collision|BreakHitResult _outhit)) "None"))))))))

(event Input|KeyboardEvents|MotionControllerLeftTrigger
  (params (Key :type Key%20Structure))
  (bind _arrow (Variables|Default|GetArrow))
  (bind _returnvalue (Transformation|GetWorldLocation _arrow))
  (:Pressed
    (if (Utilities|IsValid (stale EventPickup AttachTo))
      (if (Utilities|Name|Equal(Name) (Variables|/Script/HeadMountedDisplay.MotionControllerComponent|GetMotionSource (stale EventPickup _asmotion_controller_component)) "EControllerHand::Left")
        (if true
          (bind (_outhit _returnvalue_2) (Collision|LineTraceByChannel _returnvalue (+ _returnvalue (* (Math|Vector|GetForwardVector _arrow) 3e+03)) "TraceTypeQuery1" false 0 "ForDuration"))
          (if _returnvalue_2
            (Game|Damage|ApplyPointDamage (.HitActor (Collision|BreakHitResult _outhit)) 1.0 (.ImpactPoint (Collision|BreakHitResult _outhit)) _outhit)
            (Audio|PlaySoundatLocation "/Game/MiniGame1/Audio/Sound_Effects/Beretta_M9.Beretta_M9" (.ImpactPoint (Collision|BreakHitResult _outhit)) "0, 0, 0" 0.2 1.0 0.0 0 0 0)
            (if (Physics|IsSimulatingPhysics (.HitComponent (Collision|BreakHitResult _outhit)) "None")
              (Physics|AddImpulseatLocation (.HitComponent (Collision|BreakHitResult _outhit)) (.ImpactPoint (Collision|BreakHitResult _outhit)) (.ImpactPoint (Collision|BreakHitResult _outhit)) "None"))))))))

(fn ConstructionScript)