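; VR handgun that attaches to a motion controller on pickup and fires hitscan shots from that hand's trigger.
; Shots line-trace from an arrow, applying point damage, an impact sound and impulses to physics objects.
; Tilting the mesh's up vector near vertical blocks firing and refills up to eight rounds via a Tick-driven Delay.
; That reload state also swaps the hologram sight material and reveals the per-round ammo display.
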(event EventBeginPlay
  (Rendering|SetVisibility (Variables|Default|Getsights) false false))

(event EventTick
  (params (DeltaSeconds :type Float%20%28single-precision%29))
  (bind _staticmeshcomponent (Variables|Debug|GetStaticMeshComponent))
  (bind _returnvalue (Math|Vector|GetUpVector _staticmeshcomponent))
  (bind _z (Math|Vector|BreakVector _returnvalue))
  (bind _returnvalue_2 (< _z 0.75))
  (bind _returnvalue_3 (> _z -0.75))
  (bind _returnvalue_4 (and _returnvalue_3 _returnvalue_2))
  (bind _returnvalue_5 (Math|Boolean|NotEqual(Boolean) _returnvalue_4 true))
  (Variables|Default|SetReLoading _returnvalue_5)
  (Rendering|Material|SetMaterial (Variables|Default|Getsights) 0 (select _returnvalue_5 "/Game/HubWorld/Materials/M_Hologram_Inst_Inst.M_Hologram_Inst_Inst" "/Game/HubWorld/Materials/M_Hologram_Inst_Inst3_Inst.M_Hologram_Inst_Inst3_Inst"))
  (Utilities|FlowControl|Sequence
    (:then_0
      (if (Variables|Default|GetReLoading)
        (if (< (Variables|Default|GetRounds) 8.0)
          (Utilities|FlowControl|Delay 0.5)
          (if (Variables|Default|GetReLoading)
            (Variables|Default|SetRounds (+ (Variables|Default|GetRounds) 1.0))))))
    (:then_1
      ;[1 1 1] Ammo Display
      (Rendering|SetVisibility (Variables|Default|GetAmmo1) (and (>= (Variables|Default|GetRounds) 1.0) (Variables|Default|GetReLoading)) false)
      (Rendering|SetVisibility (Variables|Default|GetAmmo2) (and (>= (Variables|Default|GetRounds) 2.0) (Variables|Default|GetReLoading)) false)
      (Rendering|SetVisibility (Variables|Default|GetAmmo3) (and (>= (Variables|Default|GetRounds) 3.0) (Variables|Default|GetReLoading)) false)
      (Rendering|SetVisibility (Variables|Default|GetAmmo4) (and (>= (Variables|Default|GetRounds) 4.0) (Variables|Default|GetReLoading)) false)
      (Rendering|SetVisibility (Variables|Default|GetAmmo5) (and (>= (Variables|Default|GetRounds) 5.0) (Variables|Default|GetReLoading)) false)
      (Rendering|SetVisibility (Variables|Default|GetAmmo6) (and (>= (Variables|Default|GetRounds) 6.0) (Variables|Default|GetReLoading)) false)
      (Rendering|SetVisibility (Variables|Default|GetAmmo7) (and (>= (Variables|Default|GetRounds) 7.0) (Variables|Default|GetReLoading)) false)
      (Rendering|SetVisibility (Variables|Default|GetAmmo8) (and (>= (Variables|Default|GetRounds) 8.0) (Variables|Default|GetReLoading)) false))))

(event EventPickup
  (params (AttachTo :type Scene%20Component%20Object%20Reference))
  (bind _ammogroup (Variables|Default|Getammogroup))
  (if (Utilities|IsValid AttachTo)
    (bind _asmotion_controller_component (Utilities|Casting|CastToMotionControllerComponent AttachTo))
    (Variables|Default|Setpicked_up true)
    (Physics|SetSimulatePhysics (Variables|Debug|GetStaticMeshComponent) false)
    (Transformation|AttachComponentToComponent (VehicleSound|GetRootComponent) AttachTo "None" "SnapToTarget" "SnapToTarget" "KeepWorld" false)
    (Transformation|SetRelativeLocationAndRotation (Variables|Debug|GetStaticMeshComponent) "3.000000,0.000000,-2.000000" "-20.000000,0.000000,90.000000" false false)
    (Rendering|SetVisibility (Variables|Default|Getsights) true false)
    (if (Utilities|Name|Equal(Name) (Variables|/Script/HeadMountedDisplay.MotionControllerComponent|GetMotionSource _asmotion_controller_component) "EControllerHand::Right")
      (Transformation|SetRelativeLocationAndRotation _ammogroup "-3.000000,-2.000000,-1.000000" "0, 0, 0" false false)
      (else
        (Transformation|SetRelativeLocationAndRotation _ammogroup "-3.000000,-2.000000,1.000000" "-0.000000,0.000000,0.000000" false false)))))

(event EventDrop
  (Variables|Default|Setpicked_up false)
  (Physics|SetSimulatePhysics (Variables|Debug|GetStaticMeshComponent) true)
  (Transformation|DetachFromActor "KeepWorld" "KeepWorld" "KeepWorld")
  (Rendering|SetVisibility (Variables|Default|Getsights) false false))

(event Input|KeyboardEvents|MotionControllerRightTrigger
  (params (Key :type Key%20Structure))
  (bind _arrow (Variables|Default|GetArrow))
  (bind _returnvalue (Transformation|GetWorldLocation _arrow))
  (:Pressed
    (if (Utilities|IsValid (stale EventPickup AttachTo))
      (if (Utilities|Name|Equal(Name) (Variables|/Script/HeadMountedDisplay.MotionControllerComponent|GetMotionSource (stale EventPickup _asmotion_controller_component)) "EControllerHand::Right")
        (if (Variables|Default|Getpicked_up)
          (if (> (Variables|Default|GetRounds) 0.0)
            (if (not (Variables|Default|GetReLoading))
              (bind (_outhit _returnvalue_2) (Collision|LineTraceByChannel _returnvalue (+ _returnvalue (* (Math|Vector|GetForwardVector _arrow) 3e+03)) "TraceTypeQuery1" false 0 "ForDuration"))
              (Variables|Default|SetRounds (- (Variables|Default|GetRounds) 1.0))
              (if _returnvalue_2
                (Game|Damage|ApplyPointDamage (.HitActor (Collision|BreakHitResult _outhit)) 1.0 (.ImpactPoint (Collision|BreakHitResult _outhit)) _outhit)
                (Audio|PlaySoundatLocation "/Game/MiniGame1/Audio/Sound_Effects/Beretta_M9.Beretta_M9" (.ImpactPoint (Collision|BreakHitResult _outhit)) "0, 0, 0" 0.2 1.0 0.0 0 0 0)
                (if (Physics|IsSimulatingPhysics (.HitComponent (Collision|BreakHitResult _outhit)) "None")
                  (Physics|AddImpulseatLocation (.HitComponent (Collision|BreakHitResult _outhit)) (.ImpactPoint (Collision|BreakHitResult _outhit)) (.ImpactPoint (Collision|BreakHitResult _outhit)) "None"))))))))))

(event Input|KeyboardEvents|MotionControllerLeftTrigger
  (params (Key :type Key%20Structure))
  (bind _arrow (Variables|Default|GetArrow))
  (bind _returnvalue (Transformation|GetWorldLocation _arrow))
  (:Pressed
    (if (Utilities|IsValid (stale EventPickup AttachTo))
      (if (Utilities|Name|Equal(Name) (Variables|/Script/HeadMountedDisplay.MotionControllerComponent|GetMotionSource (stale EventPickup _asmotion_controller_component)) "EControllerHand::Left")
        (if (Variables|Default|Getpicked_up)
          (if (> (Variables|Default|GetRounds) 0.0)
            (if (not (Variables|Default|GetReLoading))
              (bind (_outhit _returnvalue_2) (Collision|LineTraceByChannel _returnvalue (+ _returnvalue (* (Math|Vector|GetForwardVector _arrow) 3e+03)) "TraceTypeQuery1" false 0 "ForDuration"))
              (Variables|Default|SetRounds (- (Variables|Default|GetRounds) 1.0))
              (if _returnvalue_2
                (Game|Damage|ApplyPointDamage (.HitActor (Collision|BreakHitResult _outhit)) 1.0 (.ImpactPoint (Collision|BreakHitResult _outhit)) _outhit)
                (Audio|PlaySoundatLocation "/Game/MiniGame1/Audio/Sound_Effects/Beretta_M9.Beretta_M9" (.ImpactPoint (Collision|BreakHitResult _outhit)) "0, 0, 0" 0.2 1.0 0.0 0 0 0)
                (if (Physics|IsSimulatingPhysics (.HitComponent (Collision|BreakHitResult _outhit)) "None")
                  (Physics|AddImpulseatLocation (.HitComponent (Collision|BreakHitResult _outhit)) (.ImpactPoint (Collision|BreakHitResult _outhit)) (.ImpactPoint (Collision|BreakHitResult _outhit)) "None"))))))))))

(fn ConstructionScript)