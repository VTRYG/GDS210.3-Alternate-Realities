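; Gun_BP is a VR pistol for MiniGame1 that can be picked up, dropped and fired with motion controllers.
; Pickup disables physics and snaps the gun to the given component with a fixed mesh offset, while Drop detaches it and restores physics.
; While held, either trigger line-traces from the Arrow with debug drawing, applies point damage and an impulse using the impact point as its vector, then plays a gunshot.
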(event EventBeginPlay)

(event Collision|EventActorBeginOverlap
  (params (OtherActor :type Actor%20Object%20Reference)))

(event EventTick
  (params (DeltaSeconds :type Float%20%28single-precision%29)))

(event EventPickup
  (params (AttachTo :type Scene%20Component%20Object%20Reference))
  (Variables|Default|Setpicked_up true)
  (Physics|SetSimulatePhysics (Variables|Debug|GetStaticMeshComponent) false)
  (Transformation|AttachComponentToComponent (VehicleSound|GetRootComponent) AttachTo "None" "SnapToTarget" "SnapToTarget" "KeepWorld" false)
  (Transformation|SetRelativeLocationAndRotation (Variables|Debug|GetStaticMeshComponent) "3.000000,-0.999999,1.000001" "0, 0,90.000076" false false))

(event EventDrop
  (Variables|Default|Setpicked_up false)
  (Physics|SetSimulatePhysics (Variables|Debug|GetStaticMeshComponent) true)
  (Transformation|DetachFromActor "KeepWorld" "KeepWorld" "KeepWorld"))

(event Input|KeyboardEvents|MotionControllerRightTrigger
  (params (Key :type Key%20Structure))
  (bind _arrow (Variables|Default|GetArrow))
  (bind _returnvalue (Transformation|GetWorldLocation _arrow))
  (:Pressed
    (if (Variables|Default|Getpicked_up)
      (bind _outhit (Collision|LineTraceByChannel _returnvalue (+ (* (Math|Vector|GetForwardVector _arrow) 3e+03) _returnvalue) "TraceTypeQuery1" false 0 "ForDuration"))
      (Game|Damage|ApplyPointDamage (.HitActor (Collision|BreakHitResult _outhit)) 1.0 (.ImpactPoint (Collision|BreakHitResult _outhit)) _outhit)
      (Physics|AddImpulseatLocation (.HitComponent (Collision|BreakHitResult _outhit)) (.ImpactPoint (Collision|BreakHitResult _outhit)) (.ImpactPoint (Collision|BreakHitResult _outhit)) "None")
      (Audio|PlaySoundatLocation "/Game/MiniGame1/sounds/Beretta_M9.Beretta_M9" (Transformation|GetActorLocation) "0, 0, 0" 1.0 1.0 0.0 0 0 0))))

(event Input|KeyboardEvents|MotionControllerLeftTrigger
  (params (Key :type Key%20Structure))
  (bind _arrow (Variables|Default|GetArrow))
  (bind _returnvalue (Transformation|GetWorldLocation _arrow))
  (:Pressed
    (if (Variables|Default|Getpicked_up)
      (bind _outhit (Collision|LineTraceByChannel _returnvalue (+ (* (Math|Vector|GetForwardVector _arrow) 3e+03) _returnvalue) "TraceTypeQuery1" false 0 "ForDuration"))
      (Game|Damage|ApplyPointDamage (.HitActor (Collision|BreakHitResult _outhit)) 1.0 (.ImpactPoint (Collision|BreakHitResult _outhit)) _outhit)
      (Physics|AddImpulseatLocation (.HitComponent (Collision|BreakHitResult _outhit)) (.ImpactPoint (Collision|BreakHitResult _outhit)) (.ImpactPoint (Collision|BreakHitResult _outhit)) "None")
      (Audio|PlaySoundatLocation "/Game/MiniGame1/sounds/Beretta_M9.Beretta_M9" (Transformation|GetActorLocation) "0, 0, 0" 1.0 1.0 0.0 0 0 0))))

(fn ConstructionScript)